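; Player-tilted water bucket that follows the Character's rotation, spilling when tipped too far and draining steadily over time.
; MoveRight adds clamped roll, while Tick drives the left/right spill FX and re-centres the tilt.
; Six stacked water slab actors shrink and hide in sequence, recolouring the bucket green, yellow, then red.
; AddWater tops up or restores one slab per call; several unconnected legacy movement and vanishing graphs remain.
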(event EventTick
  (params (DeltaSeconds :type Float%20%28single-precision%29))
  (bind _returnvalue (Transformation|GetActorRotation))
  (bind _returnvalue_2 (Transformation|GetActorRotation))
  (bind _waterbeinguseduprate (Variables|Default|GetWaterBeingUsedupRate))
  (bind _staticmesh (Variables|Default|GetStaticMesh))
  (bind _water4 (Variables|Default|GetWater4))
  (bind _water5 (Variables|Default|GetWater5))
  (bind _water6 (Variables|Default|GetWater6))
  (bind _water3 (Variables|Default|GetWater3))
  (bind _water4_2 (Variables|Default|GetWater4))
  (bind _waterbeinguseduprate_2 (Variables|Default|GetWaterBeingUsedupRate))
  (bind _water5_2 (Variables|Default|GetWater5))
  (bind _scalereductionrate (Variables|Default|GetScaleReductionRate))
  (bind _waterbeinguseduprate_3 (Variables|Default|GetWaterBeingUsedupRate))
  (bind _waterbeinguseduprate_4 (Variables|Default|GetWaterBeingUsedupRate))
  (bind _water1 (Variables|Default|GetWater1))
  (bind _waterbeinguseduprate_5 (Variables|Default|GetWaterBeingUsedupRate))
  (bind _water2 (Variables|Default|GetWater2))
  (bind _waterbeinguseduprate_6 (Variables|Default|GetWaterBeingUsedupRate))
  (bind _water3_2 (Variables|Default|GetWater3))
  (bind _staticmesh_2 (Variables|Default|GetStaticMesh))
  (bind _water1_2 (Variables|Default|GetWater1))
  (bind _water1_3 (Variables|Default|GetWater1))
  (bind _water2_2 (Variables|Default|GetWater2))
  (bind _water2_3 (Variables|Default|GetWater2))
  (bind _water3_3 (Variables|Default|GetWater3))
  (bind _water4_3 (Variables|Default|GetWater4))
  (bind _water5_3 (Variables|Default|GetWater5))
  (bind _water6_2 (Variables|Default|GetWater6))
  (bind _water6_3 (Variables|Default|GetWater6))
  (bind _staticmesh_3 (Variables|Default|GetStaticMesh))
  (bind _scalereductionrate_2 (Variables|Default|GetScaleReductionRate))
  (bind _scalereductionrate_3 (Variables|Default|GetScaleReductionRate))
  (bind _scalereductionrate_4 (Variables|Default|GetScaleReductionRate))
  (bind _scalereductionrate_5 (Variables|Default|GetScaleReductionRate))
  (bind _scalereductionrate_6 (Variables|Default|GetScaleReductionRate))
  (bind _returnvalue_3 (Class|Actor|GetActorRelativeScale3D _water3))
  (bind _returnvalue_4 (Class|Actor|GetActorRelativeScale3D _water4))
  (bind _returnvalue_5 (Class|Actor|GetActorRelativeScale3D _water4))
  (bind _returnvalue_6 (Class|Actor|GetActorRelativeScale3D _water5))
  (bind _returnvalue_7 (Class|Actor|GetActorRelativeScale3D _water5))
  (bind _returnvalue_8 (Class|Actor|GetActorRelativeScale3D _water1))
  (bind _returnvalue_9 (Class|Actor|GetActorRelativeScale3D _water1))
  (bind _returnvalue_10 (Class|Actor|GetActorRelativeScale3D _water2))
  (bind _returnvalue_11 (Class|Actor|GetActorRelativeScale3D _water2))
  (bind _returnvalue_12 (Class|Actor|GetActorRelativeScale3D _water3_2))
  (bind _returnvalue_13 (Class|Actor|GetActorRelativeScale3D _water3_2))
  (bind _returnvalue_14 (Class|Actor|GetActorRelativeScale3D _water6_3))
  (bind _returnvalue_15 (Class|Actor|GetActorRelativeScale3D _water6_2))
  (bind _returnvalue_16 (Class|Actor|GetActorRelativeScale3D _water4_3))
  (bind _returnvalue_17 (Class|Actor|GetActorRelativeScale3D _water4_2))
  (bind _returnvalue_18 (Class|Actor|GetActorRelativeScale3D _water5_3))
  (bind _returnvalue_19 (Class|Actor|GetActorRelativeScale3D _water5_2))
  (bind _returnvalue_20 (Class|Actor|GetActorRelativeScale3D _water1_2))
  (bind _returnvalue_21 (Class|Actor|GetActorRelativeScale3D _water1_3))
  (bind _returnvalue_22 (Class|Actor|GetActorRelativeScale3D _water2_2))
  (bind _returnvalue_23 (Class|Actor|GetActorRelativeScale3D _water2_3))
  (bind _returnvalue_24 (Class|Actor|GetActorRelativeScale3D _water3_3))
  (bind _returnvalue_25 (Class|Actor|GetActorRelativeScale3D _water6))
  (bind (_roll _pitch _yaw) (Math|Rotator|BreakRotator _returnvalue_2))
  (bind _returnvalue_26 (Class|Actor|GetActorRelativeScale3D _water6))
  (bind _returnvalue_27 (- (.z _returnvalue_14) _scalereductionrate))
  (bind _returnvalue_28 (- (.z _returnvalue_4) _waterbeinguseduprate_2))
  (bind _returnvalue_29 (- (.z _returnvalue_6) _waterbeinguseduprate_3))
  (bind _returnvalue_30 (- (.z _returnvalue_8) _waterbeinguseduprate_4))
  (bind _returnvalue_31 (- (.z _returnvalue_10) _waterbeinguseduprate_5))
  (bind _returnvalue_32 (- (.z _returnvalue_12) _waterbeinguseduprate_6))
  (bind _returnvalue_33 (- (.z _returnvalue_16) _scalereductionrate_5))
  (bind _returnvalue_34 (- (.z _returnvalue_18) _scalereductionrate_6))
  (bind _returnvalue_35 (- (.z _returnvalue_20) _scalereductionrate_2))
  (bind _returnvalue_36 (- (.z _returnvalue_22) _scalereductionrate_3))
  (bind _returnvalue_37 (- (.z _returnvalue_24) _scalereductionrate_4))
  (bind _returnvalue_38 (- (.z _returnvalue_26) _waterbeinguseduprate))
  (Utilities|FlowControl|Sequence
    (:then_0
      ;[1 1 1] Water Falls
      (Math|Float|CompareFloat (Variables|Default|Getrot) -3e+01
        (:>
          (Math|Float|CompareFloat (Variables|Default|Getrot) 3e+01
            (:>
              (Components|Activation|Activate (Variables|/Game/Bucket/WaterPartFXBP.WaterPartFXBP_C|GetParticleSystem (Variables|Default|GetRightSpillFx)) false :!label _label))
            (:==
              (goto _label))
            (:<
              (Components|Activation|Deactivate (Variables|/Game/Bucket/WaterPartFXBP.WaterPartFXBP_C|GetParticleSystem (Variables|Default|GetLeftSpillFx)))
              (Components|Activation|Deactivate (Variables|/Game/Bucket/WaterPartFXBP.WaterPartFXBP_C|GetParticleSystem (Variables|Default|GetRightSpillFx))))))
        (:==
          (Components|Activation|Activate (Variables|/Game/Bucket/WaterPartFXBP.WaterPartFXBP_C|GetParticleSystem (Variables|Default|GetLeftSpillFx)) false :!label _label_2))
        (:<
          (goto _label_2))))
    (:then_1
      ;[1 1 1] Water scaling down and vanishing in sequece
      (Math|Float|CompareFloat (.roll _returnvalue) 3e+01
        (:>
          _)
        (:<
          (Math|Float|CompareFloat (.roll _returnvalue) -3e+01
            (:<
              _))))
      (Utilities|FlowControl|Sequence
        (:then_0
          (if (Variables|Default|GetWaterSlab1Active)
            (Utilities|FlowControl|Sequence
              (:then_0
                (Transformation|SetActorRelativeScale3D (Variables|Default|GetWater1) (Math|Vector|MakeVector (.x _returnvalue_20) (.y _returnvalue_20) _returnvalue_35)))
              (:then_1
                (Math|Float|CompareFloat _returnvalue_35 1.0
                  (:<
                    (Variables|Default|SetWaterSlab1Active false)
                    (Rendering|SetActorHiddenInGame _water1_3 true)
                    (Transformation|SetActorRelativeScale3D _water1_3 (Math|Vector|MakeVector (.x _returnvalue_21) (.y _returnvalue_21) 8.0))))))))
        (:then_1
          (if (Class|KismetMathLibrary|XORBoolean (Variables|Default|GetWaterSlab1Active) (Variables|Default|GetWaterSlab2Active))
            (Utilities|FlowControl|Sequence
              (:then_0
                (Transformation|SetActorRelativeScale3D (Variables|Default|GetWater2) (Math|Vector|MakeVector (.x _returnvalue_22) (.y _returnvalue_22) _returnvalue_36)))
              (:then_1
                (Math|Float|CompareFloat _returnvalue_36 1.0
                  (:<
                    (Variables|Default|SetWaterSlab2Active false)
                    (Rendering|SetActorHiddenInGame _water2_3 true)
                    (Transformation|SetActorRelativeScale3D _water2_3 (Math|Vector|MakeVector (.x _returnvalue_23) (.y _returnvalue_23) 8.0))))))))
        (:then_2
          (if (Class|KismetMathLibrary|XORBoolean (Variables|Default|GetWaterSlab2Active) (Variables|Default|GetWaterSlab3Active))
            (Utilities|FlowControl|Sequence
              (:then_0
                (Transformation|SetActorRelativeScale3D (Variables|Default|GetWater3) (Math|Vector|MakeVector (.x _returnvalue_24) (.y _returnvalue_24) _returnvalue_37)))
              (:then_1
                (Math|Float|CompareFloat _returnvalue_37 1.0
                  (:<
                    (Variables|Default|SetWaterSlab3Active false)
                    (Rendering|SetActorHiddenInGame _water3 true)
                    (Transformation|SetActorRelativeScale3D _water3 (Math|Vector|MakeVector (.x _returnvalue_3) (.y _returnvalue_3) 8.0))))))))
        (:then_3
          (if (Class|KismetMathLibrary|XORBoolean (Variables|Default|GetWaterSlab3Active) (Variables|Default|GetWaterSlab4Active))
            (Utilities|FlowControl|Sequence
              (:then_0
                (Transformation|SetActorRelativeScale3D (Variables|Default|GetWater4) (Math|Vector|MakeVector (.x _returnvalue_16) (.y _returnvalue_16) _returnvalue_33)))
              (:then_1
                (Math|Float|CompareFloat _returnvalue_33 1.0
                  (:<
                    (Variables|Default|SetWaterSlab4Active false)
                    (Rendering|SetActorHiddenInGame _water4_2 true)
                    (Transformation|SetActorRelativeScale3D _water4_2 (Math|Vector|MakeVector (.x _returnvalue_17) (.y _returnvalue_17) 8.0))))))))
        (:then_4
          (if (Class|KismetMathLibrary|XORBoolean (Variables|Default|GetWaterSlab4Active) (Variables|Default|GetWaterSlab5Active))
            (Utilities|FlowControl|Sequence
              (:then_0
                (Transformation|SetActorRelativeScale3D (Variables|Default|GetWater5) (Math|Vector|MakeVector (.x _returnvalue_18) (.y _returnvalue_18) _returnvalue_34)))
              (:then_1
                (Math|Float|CompareFloat _returnvalue_34 1.0
                  (:<
                    (Variables|Default|SetWaterSlab5Active false)
                    (Rendering|SetActorHiddenInGame _water5_2 true)
                    (Transformation|SetActorRelativeScale3D _water5_2 (Math|Vector|MakeVector (.x _returnvalue_19) (.y _returnvalue_19) 8.0))))))))
        (:then_5
          (if (Class|KismetMathLibrary|XORBoolean (Variables|Default|GetWaterSlab5Active) (Variables|Default|GetWaterSlab6Active))
            (Utilities|FlowControl|Sequence
              (:then_0
                (Transformation|SetActorRelativeScale3D (Variables|Default|GetWater6) (Math|Vector|MakeVector (.x _returnvalue_14) (.y _returnvalue_14) _returnvalue_27)))
              (:then_1
                (Math|Float|CompareFloat _returnvalue_27 1.0
                  (:<
                    (Variables|Default|SetWaterSlab6Active false)
                    (Rendering|SetActorHiddenInGame _water6_2 true)
                    (Transformation|SetActorRelativeScale3D _water6_2 (Math|Vector|MakeVector (.x _returnvalue_15) (.y _returnvalue_15) 8.0))))))))))
    (:then_2
      ;[1 1 1] Re-orient the bucket back after it has been rotated by user input, and reset variable rot
      (Utilities|FlowControl|Sequence
        (:then_1
          (Math|Float|CompareFloat (stale Input|AxisEvents|InputAxisMoveRight AxisValue) 0.0
            (:>
              (goto _label_3 Reset))
            (:==
              (Utilities|FlowControl|DoOnce false :!label _label_3
                (:Completed
                  (Transformation|SetActorRotation (Math|Rotator|MakeRotator 0.0 _pitch _yaw))
                  (Variables|Default|Setrot (- (Variables|Default|Getrot) (Variables|Default|Getrot))))))
            (:<
              (goto _label_3 Reset))))))
    (:then_3
      ;[1 1 1] Reduce the water with the distance travelled by the character (signifying he uses up the water while running)
      (if (Variables|Default|GetWaterSlab1Active)
        (Utilities|FlowControl|Delay (Variables|Default|GetWaterScaleReductionDelayRate))
        (Utilities|FlowControl|Sequence
          (:then_0
            (Transformation|SetActorRelativeScale3D _water1 (Math|Vector|MakeVector (.x _returnvalue_8) (.y _returnvalue_8) _returnvalue_30)))
          (:then_1
            (Math|Float|CompareFloat _returnvalue_30 1.0
              (:<
                (Variables|Default|SetWaterSlab1Active false)
                (Rendering|SetActorHiddenInGame _water1 true)
                (Transformation|SetActorRelativeScale3D _water1 (Math|Vector|MakeVector (.x _returnvalue_9) (.y _returnvalue_9) 8.0))))))
        (elif (Variables|Default|GetWaterSlab2Active)
          (Utilities|FlowControl|Delay (Variables|Default|GetWaterScaleReductionDelayRate))
          (Utilities|FlowControl|Sequence
            (:then_0
              (Transformation|SetActorRelativeScale3D _water2 (Math|Vector|MakeVector (.x _returnvalue_10) (.y _returnvalue_10) _returnvalue_31)))
            (:then_1
              (Math|Float|CompareFloat _returnvalue_31 1.0
                (:<
                  (Variables|Default|SetWaterSlab2Active false)
                  (Rendering|SetActorHiddenInGame _water2 true)
                  (Transformation|SetActorRelativeScale3D _water2 (Math|Vector|MakeVector (.x _returnvalue_11) (.y _returnvalue_11) 8.0))))))
          (elif (Variables|Default|GetWaterSlab3Active)
            (Utilities|FlowControl|Delay (Variables|Default|GetWaterScaleReductionDelayRate))
            (Utilities|FlowControl|Sequence
              (:then_0
                (Transformation|SetActorRelativeScale3D _water3_2 (Math|Vector|MakeVector (.x _returnvalue_12) (.y _returnvalue_12) _returnvalue_32)))
              (:then_1
                (Math|Float|CompareFloat _returnvalue_32 1.0
                  (:<
                    (Variables|Default|SetWaterSlab3Active false)
                    (Rendering|SetActorHiddenInGame _water3_2 true)
                    (Transformation|SetActorRelativeScale3D _water3_2 (Math|Vector|MakeVector (.x _returnvalue_13) (.y _returnvalue_13) 8.0))))))
            (elif (Variables|Default|GetWaterSlab4Active)
              (Utilities|FlowControl|Delay (Variables|Default|GetWaterScaleReductionDelayRate))
              (Utilities|FlowControl|Sequence
                (:then_0
                  (Transformation|SetActorRelativeScale3D _water4 (Math|Vector|MakeVector (.x _returnvalue_4) (.y _returnvalue_4) _returnvalue_28)))
                (:then_1
                  (Math|Float|CompareFloat _returnvalue_28 1.0
                    (:<
                      (Variables|Default|SetWaterSlab4Active false)
                      (Rendering|SetActorHiddenInGame _water4 true)
                      (Transformation|SetActorRelativeScale3D _water4 (Math|Vector|MakeVector (.x _returnvalue_5) (.y _returnvalue_5) 8.0))))))
              (elif (Variables|Default|GetWaterSlab5Active)
                (Utilities|FlowControl|Delay (Variables|Default|GetWaterScaleReductionDelayRate))
                (Utilities|FlowControl|Sequence
                  (:then_0
                    (Transformation|SetActorRelativeScale3D _water5 (Math|Vector|MakeVector (.x _returnvalue_6) (.y _returnvalue_6) _returnvalue_29)))
                  (:then_1
                    (Math|Float|CompareFloat _returnvalue_29 1.0
                      (:<
                        (Variables|Default|SetWaterSlab5Active false)
                        (Rendering|SetActorHiddenInGame _water5 true)
                        (Transformation|SetActorRelativeScale3D _water5 (Math|Vector|MakeVector (.x _returnvalue_7) (.y _returnvalue_7) 8.0))))))
                (elif (Variables|Default|GetWaterSlab6Active)
                  (Utilities|FlowControl|Delay (Variables|Default|GetWaterScaleReductionDelayRate))
                  (Utilities|FlowControl|Sequence
                    (:then_0
                      (Transformation|SetActorRelativeScale3D _water6 (Math|Vector|MakeVector (.x _returnvalue_26) (.y _returnvalue_26) _returnvalue_38)))
                    (:then_1
                      (Math|Float|CompareFloat _returnvalue_38 1.0
                        (:<
                          (Variables|Default|SetWaterSlab6Active false)
                          (Rendering|SetActorHiddenInGame _water6 true)
                          (Transformation|SetActorRelativeScale3D _water6 (Math|Vector|MakeVector (.x _returnvalue_25) (.y _returnvalue_25) 8.0)))))))))))))
    (:then_4
      ;[1 1 1] Visual Color Change Based On Water level
      (if (or (Variables|Default|GetWaterSlab1Active) (Variables|Default|GetWaterSlab2Active))
        (Rendering|Material|SetMaterial _staticmesh_2 0 "/Game/FuturisticBucketMaterial/EGreen.EGreen")
        (Rendering|Material|SetMaterial _staticmesh_2 1 "/Game/FuturisticBucketMaterial/EGreen.EGreen")
        (elif (or (Variables|Default|GetWaterSlab3Active) (Variables|Default|GetWaterSlab4Active))
          (Rendering|Material|SetMaterial _staticmesh_3 0 "/Game/FuturisticBucketMaterial/EYellow.EYellow")
          (Rendering|Material|SetMaterial _staticmesh_3 1 "/Game/FuturisticBucketMaterial/EYellow.EYellow")
          (elif (or (Variables|Default|GetWaterSlab5Active) (Variables|Default|GetWaterSlab6Active))
            (Rendering|Material|SetMaterial _staticmesh 0 "/Game/FuturisticBucketMaterial/ERed.ERed")
            (Rendering|Material|SetMaterial _staticmesh 1 "/Game/FuturisticBucketMaterial/ERed.ERed")))))))

(event EventBeginPlay
  (bind _returnvalue (Transformation|GetActorLocation))
  ;[1 1 1] Enable Bucket Movement
  (Utilities|FlowControl|Sequence
    (:then_0
      ;[1 1 1] Initialization
      (Utilities|FlowControl|Sequence
        (:then_0
          (Variables|Default|SetWaterSlab1Active true))
        (:then_1
          (Variables|Default|SetWaterSlab2Active true))
        (:then_2
          (Variables|Default|SetWaterSlab3Active true))
        (:then_3
          (Variables|Default|SetWaterSlab4Active true))
        (:then_4
          (Variables|Default|SetWaterSlab5Active true))
        (:then_5
          (Variables|Default|SetWaterSlab6Active true))
        (:then_6
          (Variables|Default|SetScaleReductionRate 0.5))
        (:then_7
          (Variables|Default|SetAngularRotationRate 2.0))
        (:then_8
          (Variables|Default|SetWaterBeingUsedupRate 0.25))
        (:then_9
          (Variables|Default|SetWaterScaleReductionDelayRate 1.0))))
    (:then_1
      (Input|EnableInput (Game|GetPlayerController 0))
      (Variables|/Game/ThirdPersonBP/Blueprints/RunCharacter.RunCharacter_C|SetOutOfWater (Variables|Default|GetCharacter) false)
      ;[1 1 1] Spill FX orientation control
      (Utilities|FlowControl|Sequence
        (:then_0
          (Transformation|SetActorTransform (Variables|Default|GetLeftSpillFx) (Math|Transform|MakeTransform (+ _returnvalue "0.000000,-20.000000,20.000000") "0, 0, 0" "1,-1.000000,1")))
        (:then_1
          (Transformation|SetActorTransform (Variables|Default|GetRightSpillFx) (Math|Transform|MakeTransform (+ _returnvalue "0.000000,20.000000,20.000000") "0, 0, 0" "1.000000,-1.000000,1")))))))

(event Input|AxisEvents|InputAxisMoveForward
  (params (AxisValue :type Float%20%28single-precision%29))
  ;[1 1 1] Controller left right movement (Expendable delete if uunused)
  ;;[1 1 1] Controller Left Right Movement
)

(event Input|AxisEvents|InputAxisMoveRight
  (params (AxisValue :type Float%20%28single-precision%29))
  (bind _returnvalue (Transformation|GetActorRotation))
  (bind (_roll _pitch _yaw) (Math|Rotator|BreakRotator _returnvalue))
  ;[1 1 1] Rotate The bucket
  (Math|Float|CompareFloat AxisValue 0.0
    (:>
      _)
    (:<
      _))
  (Math|Float|CompareFloat (Variables|Default|Getrot) 6e+01
    (:<
      (Math|Float|CompareFloat (Variables|Default|Getrot) -6e+01
        (:>
          (Utilities|FlowControl|Sequence
            (:then_0
              (Variables|Default|Setrot (+ (Variables|Default|Getrot) (* AxisValue (Variables|Default|GetAngularRotationRate)))))
            (:then_1
              (Transformation|SetActorRotation (Transformation|GetActorRotation (Variables|Default|GetCharacter))))
            (:then_2
              (Transformation|SetActorRotation (Math|Rotator|MakeRotator (+ (Variables|Default|Getrot) _roll) _pitch _yaw)))))))))

(fn ConstructionScript)

(fn AddWater
  (bind _water2 (Variables|Default|GetWater2))
  (bind _water1 (Variables|Default|GetWater1))
  (bind _water3 (Variables|Default|GetWater3))
  (bind _water4 (Variables|Default|GetWater4))
  (bind _water5 (Variables|Default|GetWater5))
  (bind _water6 (Variables|Default|GetWater6))
  (bind _returnvalue (Class|Actor|GetActorRelativeScale3D _water2))
  (bind _returnvalue_2 (Class|Actor|GetActorRelativeScale3D _water3))
  (bind _returnvalue_3 (Class|Actor|GetActorRelativeScale3D _water4))
  (bind _returnvalue_4 (Class|Actor|GetActorRelativeScale3D _water5))
  (bind _returnvalue_5 (Class|Actor|GetActorRelativeScale3D _water6))
  (bind _returnvalue_6 (Class|Actor|GetActorRelativeScale3D _water1))
  (if (Variables|Default|GetWaterSlab1Active)
    (Transformation|SetActorRelativeScale3D _water1 (Math|Vector|MakeVector (.x _returnvalue_6) (.y _returnvalue_6) 8.0) :!label _label)
    (elif (Variables|Default|GetWaterSlab2Active)
      (Math|Float|CompareFloat (.z _returnvalue) 8.0
        (:>
          (Variables|Default|SetWaterSlab1Active true :!label _label_2)
          (Rendering|SetActorHiddenInGame _water1 false)
          (goto _label))
        (:==
          (goto _label_2))
        (:<
          (Transformation|SetActorRelativeScale3D _water2 (Math|Vector|MakeVector (.x _returnvalue) (.y _returnvalue) 8.0) :!label _label_3)))
      (elif (Variables|Default|GetWaterSlab3Active)
        (Math|Float|CompareFloat (.z _returnvalue_2) 8.0
          (:>
            (Variables|Default|SetWaterSlab2Active true :!label _label_4)
            (Rendering|SetActorHiddenInGame _water2 false)
            (goto _label_3))
          (:==
            (goto _label_4))
          (:<
            (Transformation|SetActorRelativeScale3D _water3 (Math|Vector|MakeVector (.x _returnvalue_2) (.y _returnvalue_2) 8.0) :!label _label_5)))
        (elif (Variables|Default|GetWaterSlab4Active)
          (Math|Float|CompareFloat (.z _returnvalue_3) 8.0
            (:>
              (Variables|Default|SetWaterSlab3Active true :!label _label_6)
              (Rendering|SetActorHiddenInGame _water3 false)
              (goto _label_5))
            (:==
              (goto _label_6))
            (:<
              (Transformation|SetActorRelativeScale3D _water4 (Math|Vector|MakeVector (.x _returnvalue_3) (.y _returnvalue_3) 8.0) :!label _label_7)))
          (elif (Variables|Default|GetWaterSlab5Active)
            (Math|Float|CompareFloat (.z _returnvalue_4) 8.0
              (:>
                (Variables|Default|SetWaterSlab4Active true :!label _label_8)
                (Rendering|SetActorHiddenInGame _water4 false)
                (goto _label_7))
              (:==
                (goto _label_8))
              (:<
                (Transformation|SetActorRelativeScale3D _water5 (Math|Vector|MakeVector (.x _returnvalue_4) (.y _returnvalue_4) 8.0) :!label _label_9)))
            (else
              (if (Variables|Default|GetWaterSlab6Active)
                (Math|Float|CompareFloat (.z _returnvalue_5) 8.0
                  (:>
                    (Variables|Default|SetWaterSlab5Active true :!label _label_10)
                    (Rendering|SetActorHiddenInGame _water5 false)
                    (goto _label_9))
                  (:==
                    (goto _label_10))
                  (:<
                    _))
                (else
                  (Variables|Default|SetWaterSlab6Active true)
                  (Rendering|SetActorHiddenInGame _water6 false)))
              (Transformation|SetActorRelativeScale3D _water6 (Math|Vector|MakeVector (.x _returnvalue_5) (.y _returnvalue_5) 8.0)))))))))