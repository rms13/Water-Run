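; WaterSurface_BP is an actor Blueprint that lets the player tilt a bucket around X through the Rotate_Right and Rotate_Left input axes.
; BeginPlay enables input from the first player controller, and each axis event calls SetActorRotation.
; Right sets roll to the negated axis value within a small clamp, zeroing pitch and yaw.
; Left adds its value to the current roll unclamped, keeping pitch and yaw.
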(event EventBeginPlay
  ;[1 1 1] Enable Bucket Movement
  (Input|EnableInput (Game|GetPlayerController 0)))

(event Collision|EventActorBeginOverlap
  (params (OtherActor :type Actor%20Object%20Reference)))

(event EventTick
  (params (DeltaSeconds :type Float%20%28single-precision%29)))

(event Input|AxisEvents|InputAxisRotate_Right
  (params (AxisValue :type Float%20%28single-precision%29))
  (bind (_roll _pitch _yaw) (Math|Rotator|BreakRotator "0, 0, 0"))
  ;[1 1 1] Right Rotate The bucket Along X
  (Transformation|SetActorRotation (Math|Rotator|MakeRotator (Math|Float|Clamp(Float) (- _roll AxisValue) -5.0 5.0) _pitch _yaw)))

(event Input|AxisEvents|InputAxisRotate_Left
  (params (AxisValue :type Float%20%28single-precision%29))
  (bind _returnvalue (Transformation|GetActorRotation))
  (bind (_roll _pitch _yaw) (Math|Rotator|BreakRotator _returnvalue))
  ;[1 1 1] Left Rotate The Bucket Alont X
  (Transformation|SetActorRotation (Math|Rotator|MakeRotator (+ AxisValue _roll) _pitch _yaw)))

(fn ConstructionScript)