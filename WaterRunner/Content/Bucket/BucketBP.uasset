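; Player-controlled bucket that moves by physics and tilts, with a spill effect actor for each side.
; Movement axes push the collider along its forward and right vectors, while the tilt axis rotates the actor about Y.
; BeginPlay places the two existing spill effects at mirrored offsets above the bucket.
; Logic to spawn the effects, reset their rotation and drive spill rate from pitch is present but disconnected.
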(event EventBeginPlay
  (bind _returnvalue (Transformation|GetActorLocation))
  (bind _returnvalue_2 (+ _returnvalue "0, 0, 0"))
  (Utilities|FlowControl|Sequence
    (:then_0
      (Transformation|SetActorTransform (Variables|Default|GetLeftSpillFx) (Math|Transform|MakeTransform (+ _returnvalue_2 "-20.000000, 0,40.000000"))))
    (:then_1
      (Transformation|SetActorTransform (Variables|Default|GetRightSpillFx) (Math|Transform|MakeTransform (+ _returnvalue_2 "20.000000, 0,40.000000") "0, 0, 0" "-1.000000,1.000000,1")))))

(event Collision|EventActorBeginOverlap
  (params (OtherActor :type Actor%20Object%20Reference)))

(event EventTick
  (params (DeltaSeconds :type Float%20%28single-precision%29)))

(event Input|AxisEvents|InputAxisMoveForward
  (params (AxisValue :type Float%20%28single-precision%29))
  (Physics|AddForce (Variables|Default|GetBucketCollider) (* (Math|Vector|GetForwardVector (Variables|Default|GetBucketCollider)) (* AxisValue 6e+02)) "None" false))

(event Input|AxisEvents|InputAxisMoveRight
  (params (AxisValue :type Float%20%28single-precision%29))
  (Physics|AddForce (Variables|Default|GetBucketCollider) (* (Math|Vector|GetRightVector (Variables|Default|GetBucketCollider)) (* AxisValue 6e+02)) "None" false))

(event Input|AxisEvents|InputAxisTiltRight
  (params (AxisValue :type Float%20%28single-precision%29))
  (Transformation|SetActorRotation (Math|Conversions|RotationFromXVector (Math|Vector|RotateVectorAroundAxis (Math|Rotator|GetRotationXVector (Transformation|GetActorRotation)) (* AxisValue 4.0) "0.000000,-1.000000,0.000000"))))

(fn ConstructionScript)