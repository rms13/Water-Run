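; Player-controllable bucket vehicle that moves by physics forces and tilts on input.
; MoveForward and MoveRight axes push BucketCollider along its forward and right vectors.
; TiltRight rotates the actor's X vector around the world Y axis and rebuilds the actor rotation from it.
; BeginPlay spawns two mirrored WaterPartFXBP actors above the bucket at opposite X offsets, without attaching them.
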(event EventBeginPlay
  (bind _returnvalue (Transformation|GetActorLocation))
  (bind _returnvalue_2 (Transformation|GetActorRotation))
  (bind _returnvalue_3 (Math|Vector|GetForwardVector _returnvalue_2))
  (bind _returnvalue_4 (Math|Vector|Normalize _returnvalue_3))
  (bind _returnvalue_5 (+ _returnvalue _returnvalue_4))
  (Utilities|FlowControl|Sequence
    (:then_0
      (Game|SpawnActorfromClass "/Game/Vehicle/Bucket/WaterPartFXBP.WaterPartFXBP_C" (Math|Transform|MakeTransform (+ _returnvalue_5 "-20.000000, 0,40.000000") _returnvalue_2) "AdjustIfPossibleButAlwaysSpawn" 0 0))
    (:then_1
      (Game|SpawnActorfromClass "/Game/Vehicle/Bucket/WaterPartFXBP.WaterPartFXBP_C" (Math|Transform|MakeTransform (+ _returnvalue_5 "20.000000, 0,40.000000") _returnvalue_2 "-1.000000,1.000000,1") "AdjustIfPossibleButAlwaysSpawn" 0 0))))

(event Collision|EventActorBeginOverlap
  (params (OtherActor :type Actor%20Object%20Reference)))

(event EventTick
  (params (DeltaSeconds :type Float%20%28single-precision%29)))

(event Input|AxisEvents|InputAxisMoveForward
  (params (AxisValue :type Float%20%28single-precision%29))
  (Physics|AddForce (Variables|Default|GetBucketCollider) (* (Math|Vector|GetForwardVector (Variables|Default|GetBucketCollider)) (* AxisValue 6e+02)) "None" false))

(event Input|AxisEvents|InputAxisMoveRight
  (params (AxisValue :type Float%20%28single-precision%29))
  (Physics|AddForce (Variables|Default|GetBucketCollider) (* (Math|Vector|GetRightVector (Variables|Default|GetBucketCollider)) (* AxisValue 6e+02)) "None" false))

(event Input|AxisEvents|InputAxisTiltRight
  (params (AxisValue :type Float%20%28single-precision%29))
  (Transformation|SetActorRotation (Math|Conversions|RotationFromXVector (Math|Vector|RotateVectorAroundAxis (Math|Rotator|GetRotationXVector (Transformation|GetActorRotation)) (* AxisValue 4.0) "0.000000,-1.000000,0.000000"))))

(fn ConstructionScript)